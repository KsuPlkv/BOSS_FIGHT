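; AI controller for the boss fight that starts and stops the boss's behavior tree.
; On BeginPlay, StartBT runs BossFight_BT, sets up the BossFight_BB blackboard and stores the controller itself under the AIController key.
; A FinishBT event stops the brain component's logic and prints a debug message.
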(event `self.ReceiveBeginPlay`
  (`self.StartBT`))

(event `StartBT`
  (`self.RunBehaviorTree` "/Game/AI/BossFight_BT.BossFight_BT")
  (bind _blackboardcomponent (`self.UseBlackboard` "/Game/AI/BossFight_BB.BossFight_BB"))
  (`BlackboardComponent.SetValueAsObject` _blackboardcomponent "AIController" self))

(event `FinishBT`
  (`BrainComponent.StopLogic` (`self.BrainComponent`) "")
  (`KismetSystemLibrary.PrintString` "stop logic"))

(fn `UserConstructionScript`)