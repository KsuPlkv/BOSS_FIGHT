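; Laser attack actor that fires a single beam toward the player and deals damage on a hit, all on BeginPlay.
; It moves to SocketLocation and sets the Niagara beam end by clamping a constant between start and latest player locations per axis, with a height offset.
; A Camera-channel line trace to that same point applies fixed damage if it hits the first-person player character.
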(event `self.ReceiveBeginPlay`
  (bind (_startplayerlocation_x _startplayerlocation_y _startplayerlocation_z) (`KismetMathLibrary.BreakVector` (`self.StartPlayerLocation`)))
  (bind (_latestplayerlocation_x _latestplayerlocation_y _latestplayerlocation_z) (`KismetMathLibrary.BreakVector` (`self.LatestPlayerLocation`)))
  (bind _returnvalue (`KismetMathLibrary.FClamp` 0.1 _startplayerlocation_x _latestplayerlocation_x))
  (bind _returnvalue_2 (`KismetMathLibrary.FClamp` 0.1 _startplayerlocation_y _latestplayerlocation_y))
  (bind _asfirst_person_character (cast `/Game/Blueprints/Player/FirstPersonCharacter` (`GameplayStatics.GetPlayerCharacter` 0) :!pure true))
  (bind _returnvalue_3 (+ (`KismetMathLibrary.FClamp` 0.1 _startplayerlocation_z _latestplayerlocation_z) 35.0))
  (`SceneComponent.K2_SetWorldLocation` (`self.DefaultSceneRoot`) (`self.SocketLocation`) false false)
  (`FXSystemComponent.SetVectorParameter` (`self.Beam_NS`) "User.Beam End" (`KismetMathLibrary.MakeVector` _returnvalue _returnvalue_2 _returnvalue_3))
  (bind _outhit (`KismetSystemLibrary.LineTraceSingle` (`self.SocketLocation`) (`KismetMathLibrary.MakeVector` _returnvalue _returnvalue_2 _returnvalue_3) "TraceTypeQuery2" false (`self.IgnoreActors`) "None" true (struct :`R` 1.0 :`A` 1.0) (struct :`G` 1.0 :`A` 1.0) 0.1))
  (if (== (`.HitActor` (`GameplayStatics.BreakHitResult` _outhit)) _asfirst_person_character)
    (`GameplayStatics.ApplyDamage` _asfirst_person_character 5.0)))

(fn `UserConstructionScript`)