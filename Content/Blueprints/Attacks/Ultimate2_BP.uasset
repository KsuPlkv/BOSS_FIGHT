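; Ultimate attack actor that rises, damages the player inside its box for several seconds, then sinks and destroys itself.
; BeginPlay sequences three phases with Delays and looping timers, pausing each timer before starting the next.
; Timer events step the root's height up or down, or damage the first player character while it overlaps Box.
; The three Paper sprites are set visible after both the rise and damage phases.
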(event `self.ReceiveBeginPlay`
  (set `self.Sprites` (`|MakeArray` (`self.PaperSprite`) (`self.PaperSprite1`) (`self.PaperSprite2`)))
  (bind _returnvalue (`KismetSystemLibrary.K2_SetTimerDelegate` (delegate `CustomEvent_0`) 0.1 true))
  (`KismetSystemLibrary.Delay` 1.0)
  (`KismetSystemLibrary.K2_PauseTimerHandle` _returnvalue)
  (for _array_element (`self.Sprites`)
    (`SceneComponent.SetVisibility` _array_element true false))
  (bind _returnvalue_2 (`KismetSystemLibrary.K2_SetTimerDelegate` (delegate `CustomEvent_1`) 0.4 true))
  (`KismetSystemLibrary.Delay` 6.0)
  (`KismetSystemLibrary.K2_PauseTimerHandle` _returnvalue_2)
  (for _array_element_2 (`self.Sprites`)
    (`SceneComponent.SetVisibility` _array_element_2 true false))
  (bind _returnvalue_3 (`KismetSystemLibrary.K2_SetTimerDelegate` (delegate `CustomEvent_2`) 0.1 true))
  (`KismetSystemLibrary.Delay` 1.0)
  (`KismetSystemLibrary.K2_PauseTimerHandle` _returnvalue_3)
  (`self.K2_DestroyActor`))

(event `CustomEvent_0`
  (bind _defaultsceneroot (`self.DefaultSceneRoot`))
  (bind (_returnvalue_x _returnvalue_y _returnvalue_z) (`KismetMathLibrary.BreakVector` (`SceneComponent.K2_GetComponentLocation` _defaultsceneroot)))
  (`SceneComponent.K2_SetWorldLocation` _defaultsceneroot (`KismetMathLibrary.MakeVector` _returnvalue_x _returnvalue_y (+ _returnvalue_z 10.0)) false false))

(event `CustomEvent_1`
  (bind _asfirst_person_character (cast `/Game/Blueprints/Player/FirstPersonCharacter` (`GameplayStatics.GetPlayerCharacter` 0) :!pure true))
  (if (`PrimitiveComponent.IsOverlappingActor` (`self.Box`) _asfirst_person_character)
    (`GameplayStatics.ApplyDamage` _asfirst_person_character 5.0)))

(event `CustomEvent_2`
  (bind _defaultsceneroot (`self.DefaultSceneRoot`))
  (bind (_returnvalue_x _returnvalue_y _returnvalue_z) (`KismetMathLibrary.BreakVector` (`SceneComponent.K2_GetComponentLocation` _defaultsceneroot)))
  (`SceneComponent.K2_SetWorldLocation` _defaultsceneroot (`KismetMathLibrary.MakeVector` _returnvalue_x _returnvalue_y (- _returnvalue_z 10.0)) false false))

(fn `UserConstructionScript`)