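; DefaultAttack3_BP is a timed rotating attack hazard that hurts the player on contact.
; On BeginPlay, a looping timer yaws the root component in small fixed increments, spinning the attack in steps.
; Four capsule components each apply the same fixed damage when the player's FirstPersonCharacter begins overlapping them.
; After a fixed delay, it pauses the timer and destroys itself.
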(event `self.ReceiveBeginPlay`
  (bind _returnvalue (`KismetSystemLibrary.K2_SetTimerDelegate` (delegate `CustomEvent_0`) 0.1 true))
  (`KismetSystemLibrary.Delay` 8.0)
  (`KismetSystemLibrary.K2_PauseTimerHandle` _returnvalue)
  (`self.K2_DestroyActor`))

(event `CustomEvent_0`
  (bind _defaultsceneroot (`self.DefaultSceneRoot`))
  (bind (_relativerotation_roll _relativerotation_pitch _relativerotation_yaw) (`KismetMathLibrary.BreakRotator` (`SceneComponent.RelativeRotation` _defaultsceneroot)))
  (`SceneComponent.K2_SetRelativeRotation` _defaultsceneroot (`KismetMathLibrary.MakeRotator` _relativerotation_roll _relativerotation_pitch (+ _relativerotation_yaw 6.0)) false false))

(event `self.Capsule.OnComponentBeginOverlap`
  (params (OverlappedComponent :type "PrimitiveComponent Object Reference") (OtherActor :type "Actor Object Reference") (OtherComp :type "PrimitiveComponent Object Reference") (OtherBodyIndex :type Integer) (bFromSweep :type Boolean) (SweepResult :type "HitResult Structure (by ref)"))
  (bind _asfirst_person_character (cast `/Game/Blueprints/Player/FirstPersonCharacter` (`GameplayStatics.GetPlayerCharacter` 0) :!pure true))
  (if (== OtherActor _asfirst_person_character)
    (`GameplayStatics.ApplyDamage` _asfirst_person_character 10.0 :!label _label)))

(event `self.Capsule1.OnComponentBeginOverlap`
  (params (OverlappedComponent :type "PrimitiveComponent Object Reference") (OtherActor :type "Actor Object Reference") (OtherComp :type "PrimitiveComponent Object Reference") (OtherBodyIndex :type Integer) (bFromSweep :type Boolean) (SweepResult :type "HitResult Structure (by ref)"))
  (if (== OtherActor (cast `/Game/Blueprints/Player/FirstPersonCharacter` (`GameplayStatics.GetPlayerCharacter` 0) :!pure true))
    (goto _label)))

(event `self.Capsule2.OnComponentBeginOverlap`
  (params (OverlappedComponent :type "PrimitiveComponent Object Reference") (OtherActor :type "Actor Object Reference") (OtherComp :type "PrimitiveComponent Object Reference") (OtherBodyIndex :type Integer) (bFromSweep :type Boolean) (SweepResult :type "HitResult Structure (by ref)"))
  (if (== OtherActor (cast `/Game/Blueprints/Player/FirstPersonCharacter` (`GameplayStatics.GetPlayerCharacter` 0) :!pure true))
    (goto _label)))

(event `self.Capsule3.OnComponentBeginOverlap`
  (params (OverlappedComponent :type "PrimitiveComponent Object Reference") (OtherActor :type "Actor Object Reference") (OtherComp :type "PrimitiveComponent Object Reference") (OtherBodyIndex :type Integer) (bFromSweep :type Boolean) (SweepResult :type "HitResult Structure (by ref)"))
  (if (== OtherActor (cast `/Game/Blueprints/Player/FirstPersonCharacter` (`GameplayStatics.GetPlayerCharacter` 0) :!pure true))
    (goto _label)))

(fn `UserConstructionScript`)