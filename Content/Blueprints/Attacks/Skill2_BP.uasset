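; Skill2_BP is a falling-stone boss attack that damages the player on overlap.
; On spawn it stamps a short-lived area decal as a warning and lifts its sphere high above that spot.
; After a delay the sphere is physics-launched straight down, with Sphere1's overlap applying damage only to the player character.
; It then calls the boss's CallFallingStonesF and destroys itself.
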(event `self.ReceiveBeginPlay`
  (bind _sphere (`self.Sphere`))
  (bind _returnvalue (`SceneComponent.K2_GetComponentLocation` (`self.DefaultSceneRoot`)))
  (`GameplayStatics.SpawnDecalAtLocation` "/Game/Materials/AreaDA_Mat.AreaDA_Mat" (150.0 150.0 150.0) _returnvalue (struct :`Pitch` -90.0) 1.4)
  (`SceneComponent.K2_SetWorldLocation` (`self.Sphere`) (`KismetMathLibrary.MakeVector` (.x _returnvalue) (.y _returnvalue) (+ (.z _returnvalue) 1200.0)) false false)
  (`KismetSystemLibrary.Delay` 1.0)
  (`PrimitiveComponent.SetSimulatePhysics` _sphere true)
  (`PrimitiveComponent.SetPhysicsLinearVelocity` _sphere (0.0 0.0 -4000.0) false "None")
  (`KismetSystemLibrary.Delay` 1.0)
  (`/Game/Blueprints/Boss/Boss_BP.FallingStonesF` (`self.Boss`))
  (`self.K2_DestroyActor`))

(event `self.Sphere1.OnComponentBeginOverlap`
  (params (OverlappedComponent :type "PrimitiveComponent Object Reference") (OtherActor :type "Actor Object Reference") (OtherComp :type "PrimitiveComponent Object Reference") (OtherBodyIndex :type Integer) (bFromSweep :type Boolean) (SweepResult :type "HitResult Structure (by ref)"))
  (bind _asfirst_person_character (cast `/Game/Blueprints/Player/FirstPersonCharacter` (`GameplayStatics.GetPlayerCharacter` 0) :!pure true))
  (if (== OtherActor _asfirst_person_character)
    (`GameplayStatics.ApplyDamage` _asfirst_person_character 40.0)))

(fn `UserConstructionScript`)