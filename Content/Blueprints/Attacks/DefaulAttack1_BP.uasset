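; DefaulAttack1_BP is a telegraphed area attack actor that damages the player.
; On BeginPlay it places a short-lived warning decal beneath the player's current position, waits, then plays a Niagara effect and sound on itself.
; IsPlayerInside then checks its Capsule for overlapping pawns once, applying fixed damage if the player is among them.
; After a brief delay it destroys itself and calls the Finished dispatcher.
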(event `self.ReceiveBeginPlay`
  (bind (_returnvalue_x _returnvalue_y _returnvalue_z) (`KismetMathLibrary.BreakVector` (`SceneComponent.K2_GetComponentLocation` (`Character.Mesh` (cast `/Game/Blueprints/Player/FirstPersonCharacter` (`GameplayStatics.GetPlayerCharacter` 0) :!pure true)))))
  (`GameplayStatics.SpawnDecalAtLocation` "/Game/Materials/AreaDA_Mat.AreaDA_Mat" (400.0 400.0 400.0) (`KismetMathLibrary.MakeVector` _returnvalue_x _returnvalue_y (- _returnvalue_z 100.0)) (struct :`Pitch` -90.0) 1.0)
  (`KismetSystemLibrary.Delay` 1.0)
  (`AddComponent|NODE_AddNiagaraComponent-0`)
  (`GameplayStatics.PlaySoundAtLocation` "/Game/Audio/Skill2_SW.Skill2_SW" (`SceneComponent.K2_GetComponentLocation` (`self.DefaultSceneRoot`)) (struct) 1.0 1.0 0.0 null null null)
  (`self.IsPlayerInside`))

(event `IsPlayerInside`
  (bind _capsule (`self.Capsule`))
  (bind _asfirst_person_character (cast `/Game/Blueprints/Player/FirstPersonCharacter` (`GameplayStatics.GetPlayerCharacter` 0) :!pure true))
  (bind _outactors (`KismetSystemLibrary.ComponentOverlapActors` _capsule (`SceneComponent.K2_GetComponentToWorld` _capsule) (`|MakeArray` "ObjectTypeQuery3" :!type "EObjectTypeQuery Enum")))
  (for _array_element _outactors
    (if (== _array_element _asfirst_person_character)
      (`GameplayStatics.ApplyDamage` _asfirst_person_character 40.0)
      (break)))
  (`KismetSystemLibrary.Delay` 0.8)
  (`self.K2_DestroyActor`)
  (`self.Finished`))

(fn `UserConstructionScript`)