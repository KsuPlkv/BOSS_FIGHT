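; Ult1 is an ultimate attack actor that spins, then explodes, damaging the first-person player on overlap with any of its four capsules.
; A looping timer rotates the root in yaw for six seconds before Explosion runs.
; Explosion recolours four cylinders through dynamic material instances, enlarges them on a timer for a second, calls Finished, flips the colour back and destroys the actor.
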(event `self.ReceiveBeginPlay`
  (bind _returnvalue (`KismetSystemLibrary.K2_SetTimerDelegate` (delegate `CustomEvent_0`) 0.1 true))
  (`KismetSystemLibrary.Delay` 6.0)
  (`KismetSystemLibrary.K2_PauseTimerHandle` _returnvalue)
  (`self.Explosion`))

(event `CustomEvent_0`
  (bind _defaultsceneroot (`self.DefaultSceneRoot`))
  (bind (_relativerotation_roll _relativerotation_pitch _relativerotation_yaw) (`KismetMathLibrary.BreakRotator` (`SceneComponent.RelativeRotation` _defaultsceneroot)))
  (`SceneComponent.K2_SetRelativeRotation` _defaultsceneroot (`KismetMathLibrary.MakeRotator` 0.0 0.0 (+ _relativerotation_yaw 11.0)) false false))

(event `Explosion`
  (`self.ChangeColour`)
  (bind _returnvalue (`KismetSystemLibrary.K2_SetTimerDelegate` (delegate `CustomEvent_2`) 0.5 true))
  (`KismetSystemLibrary.Delay` 1.0)
  (`KismetSystemLibrary.K2_PauseTimerHandle` _returnvalue)
  (`self.Finished`)
  (`self.ChangeColour`)
  (`self.K2_DestroyActor`))

(event `CustomEvent_2`
  (bind _cylinder1 (`self.Cylinder1`))
  (bind _cylinder (`self.Cylinder`))
  (bind _cylinder2 (`self.Cylinder2`))
  (bind _cylinder3 (`self.Cylinder3`))
  (bind (_relativescale3d_x _relativescale3d_y _relativescale3d_z) (`KismetMathLibrary.BreakVector` (`SceneComponent.RelativeScale3D` _cylinder1)))
  (bind (_relativescale3d_x_2 _relativescale3d_y_2 _relativescale3d_z_2) (`KismetMathLibrary.BreakVector` (`SceneComponent.RelativeScale3D` _cylinder)))
  (bind (_relativescale3d_x_3 _relativescale3d_y_3 _relativescale3d_z_3) (`KismetMathLibrary.BreakVector` (`SceneComponent.RelativeScale3D` _cylinder2)))
  (bind (_relativescale3d_x_4 _relativescale3d_y_4 _relativescale3d_z_4) (`KismetMathLibrary.BreakVector` (`SceneComponent.RelativeScale3D` _cylinder3)))
  (`SceneComponent.SetWorldScale3D` _cylinder1 (`KismetMathLibrary.MakeVector` (+ _relativescale3d_x 5.0) (+ _relativescale3d_y 5.0) (+ _relativescale3d_z 5.0)))
  (`SceneComponent.SetWorldScale3D` _cylinder (`KismetMathLibrary.MakeVector` (+ _relativescale3d_x_2 5.0) (+ _relativescale3d_y_2 5.0) (+ _relativescale3d_z_2 5.0)))
  (`SceneComponent.SetWorldScale3D` _cylinder2 (`KismetMathLibrary.MakeVector` (+ _relativescale3d_x_3 5.0) (+ _relativescale3d_y_3 5.0) (+ _relativescale3d_z_3 5.0)))
  (`SceneComponent.SetWorldScale3D` _cylinder3 (`KismetMathLibrary.MakeVector` (+ _relativescale3d_x_4 5.0) (+ _relativescale3d_y_4 5.0) (+ _relativescale3d_z_4 5.0))))

(event `self.Capsule3.OnComponentBeginOverlap`
  (params (OverlappedComponent :type "PrimitiveComponent Object Reference") (OtherActor :type "Actor Object Reference") (OtherComp :type "PrimitiveComponent Object Reference") (OtherBodyIndex :type Integer) (bFromSweep :type Boolean) (SweepResult :type "HitResult Structure (by ref)"))
  (bind _asfirst_person_character (cast `/Game/Blueprints/Player/FirstPersonCharacter` (`GameplayStatics.GetPlayerCharacter` 0) :!pure true))
  (if (== OtherActor _asfirst_person_character)
    (`GameplayStatics.ApplyDamage` _asfirst_person_character 40.0 :!label _label)))

(event `self.Capsule2.OnComponentBeginOverlap`
  (params (OverlappedComponent :type "PrimitiveComponent Object Reference") (OtherActor :type "Actor Object Reference") (OtherComp :type "PrimitiveComponent Object Reference") (OtherBodyIndex :type Integer) (bFromSweep :type Boolean) (SweepResult :type "HitResult Structure (by ref)"))
  (if (== OtherActor (cast `/Game/Blueprints/Player/FirstPersonCharacter` (`GameplayStatics.GetPlayerCharacter` 0) :!pure true))
    (goto _label)))

(event `self.Capsule.OnComponentBeginOverlap`
  (params (OverlappedComponent :type "PrimitiveComponent Object Reference") (OtherActor :type "Actor Object Reference") (OtherComp :type "PrimitiveComponent Object Reference") (OtherBodyIndex :type Integer) (bFromSweep :type Boolean) (SweepResult :type "HitResult Structure (by ref)"))
  (if (== OtherActor (cast `/Game/Blueprints/Player/FirstPersonCharacter` (`GameplayStatics.GetPlayerCharacter` 0) :!pure true))
    (goto _label)))

(event `self.Capsule1.OnComponentBeginOverlap`
  (params (OverlappedComponent :type "PrimitiveComponent Object Reference") (OtherActor :type "Actor Object Reference") (OtherComp :type "PrimitiveComponent Object Reference") (OtherBodyIndex :type Integer) (bFromSweep :type Boolean) (SweepResult :type "HitResult Structure (by ref)"))
  (if (== OtherActor (cast `/Game/Blueprints/Player/FirstPersonCharacter` (`GameplayStatics.GetPlayerCharacter` 0) :!pure true))
    (goto _label)))

(fn `ChangeColour`
  (bind _colour2 (`self.Colour2`))
  (bind _colour1 (`self.Colour1`))
  (`/Engine/EditorBlueprintResources/StandardMacros.FlipFlop`
    (:`A`
      (bind _returnvalue (`PrimitiveComponent.CreateDynamicMaterialInstance` (`self.Cylinder2`) 0 null "None"))
      (`MaterialInstanceDynamic.SetVectorParameterValue` _returnvalue "Colour" _colour2)
      (bind _returnvalue_2 (`PrimitiveComponent.CreateDynamicMaterialInstance` (`self.Cylinder1`) 0 null "None"))
      (`MaterialInstanceDynamic.SetVectorParameterValue` _returnvalue_2 "Colour" _colour2)
      (bind _returnvalue_3 (`PrimitiveComponent.CreateDynamicMaterialInstance` (`self.Cylinder`) 0 null "None"))
      (`MaterialInstanceDynamic.SetVectorParameterValue` _returnvalue_3 "Colour" _colour2)
      (bind _returnvalue_4 (`PrimitiveComponent.CreateDynamicMaterialInstance` (`self.Cylinder3`) 0 null "None"))
      (`MaterialInstanceDynamic.SetVectorParameterValue` _returnvalue_4 "Colour" _colour2))
    (:`B`
      (`MaterialInstanceDynamic.SetVectorParameterValue` _returnvalue "Colour" _colour1)
      (`MaterialInstanceDynamic.SetVectorParameterValue` _returnvalue_2 "Colour" _colour1)
      (`MaterialInstanceDynamic.SetVectorParameterValue` _returnvalue_3 "Colour" _colour1)
      (`MaterialInstanceDynamic.SetVectorParameterValue` _returnvalue_4 "Colour" _colour1))))

(fn `UserConstructionScript`)