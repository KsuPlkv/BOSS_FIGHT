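; DefaultAttack2_BP is a self-destroying area attack actor that damages the first-person player.
; On BeginPlay it spawns an area decal at its root, then after a short delay adds a Niagara effect.
; At that moment a single capsule overlap check applies damage if the player is inside, so the decal precedes the hit.
; After another brief delay it removes the decal and destroys itself.
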(event `self.ReceiveBeginPlay`
  (bind _asfirst_person_character (cast `/Game/Blueprints/Player/FirstPersonCharacter` (`GameplayStatics.GetPlayerCharacter` 0) :!pure true))
  (bind _returnvalue (`GameplayStatics.SpawnDecalAtLocation` "/Game/Materials/AreaDA_Mat.AreaDA_Mat" (100.0 100.0 100.0) (`SceneComponent.K2_GetComponentLocation` (`self.DefaultSceneRoot`)) (struct :`Pitch` -90.0) 6.0))
  (`KismetSystemLibrary.Delay` 1.0)
  (`AddComponent|NODE_AddNiagaraComponent-0`)
  (if (`PrimitiveComponent.IsOverlappingActor` (`self.Capsule`) _asfirst_person_character)
    (`GameplayStatics.ApplyDamage` _asfirst_person_character 10.0))
  (`KismetSystemLibrary.Delay` 0.4)
  (`ActorComponent.K2_DestroyComponent` _returnvalue)
  (`self.K2_DestroyActor`))

(fn `UserConstructionScript`)