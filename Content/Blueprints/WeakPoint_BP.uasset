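; WeakPoint_BP is a destructible boss weak point that amplifies damage dealt by the player.
; AnyDamage accepts only the player's FirstPersonCharacter as causer, multiplies the damage, then passes it to TakeDamage and the boss's TookDamage.
; TakeDamage reduces the weak point's own HP, capping overfilled HP at max first, destroys the actor at zero or below, and prints the remaining HP.
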(event `self.SphereCollision.OnComponentHit`
  (params (HitComponent :type "PrimitiveComponent Object Reference") (OtherActor :type "Actor Object Reference") (OtherComp :type "PrimitiveComponent Object Reference") (NormalImpulse :type "Vector Structure") (Hit :type "HitResult Structure (by ref)")))

(event `self.ReceiveAnyDamage`
  (params (Damage :type "Float (single-precision)") (DamageType :type "DamageType Object Reference") (InstigatedBy :type "Controller Object Reference") (DamageCauser :type "Actor Object Reference"))
  (if (== DamageCauser (cast `/Game/Blueprints/Player/FirstPersonCharacter` (`GameplayStatics.GetPlayerCharacter` 0) :!pure true))
    (bind _output_get (set `self.WPDamage` (* Damage 6.0)))
    (`self.TakeDamage` _output_get self)
    (`/Game/Blueprints/Boss/Boss_BP.TookDamage` (`self.BossCharacter`) _output_get)))

(fn `TakeDamage`
  (params (Damage :type "Float (double-precision)") (CurrentWeakPoint :type "Actor Object Reference"))
  (if (> (`self.CurrentHP_WP`) (`self.MaxHP_WP`))
    (set `self.CurrentHP_WP` (- (`self.MaxHP_WP`) Damage))
    (else
      (set `self.CurrentHP_WP` (- (`self.CurrentHP_WP`) Damage))))
  (if (<= (`self.CurrentHP_WP`) 0.0)
    (`self.K2_DestroyActor` CurrentWeakPoint))
  (`KismetSystemLibrary.PrintString` (`KismetStringLibrary.Conv_DoubleToString` (`self.CurrentHP_WP`))))

(fn `UserConstructionScript`)